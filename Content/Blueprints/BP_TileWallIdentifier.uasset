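; Tile tool that detects which sides of the target tile actors have walls and exports the results as a Data Table CSV.
; IdentifyTileWalls fires line traces along the four world compass directions, counting a wall when the trace hits the tile itself.
; Export rotates each tile through 90° steps, records walls per rotation, resets it, then saves to TileDataTableCSVs in the project directory.
; Numbered events also preview, test and flush debug trace lines.
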(event Custom|4%20-%20Export%20Values%20to%20CSV
  (Utilities|Array|Clear (Variables|Default|GetTileWallValues)) ; Ensures Tile Wall Values Array is Empty
  (for _array_element (Variables|Default|GetTargetTileActors)
    ;[1 1 1] Calculate Wall Values at Default Tile Rotation
    (bind (_bisnorthwall_ _biseastwall_ _bissouthwall_ _biswestwall_) (CallFunction|IdentifyTileWalls _array_element (+ (Transformation|GetActorLocation _array_element) (Math|Vector|MakeVector 0.0 0.0 (Variables|Default|GetZAxisLineTraceOffset))) "ForDuration"))
    (Utilities|Array|Add (Variables|Default|GetTileWallValues) (Utilities|Struct|MakeTileDataStructure (Utilities|GetDisplayName _array_element) (Utilities|GetClass _array_element) _bisnorthwall_ _biseastwall_ _bissouthwall_ _biswestwall_ 0))
    ;[1 1 1] Calculate Wall Values at 90° Rotation
    (Transformation|SetActorRotation _array_element "0,90.000000, 0")
    (bind (_bisnorthwall__2 _biseastwall__2 _bissouthwall__2 _biswestwall__2) (CallFunction|IdentifyTileWalls _array_element (+ (Transformation|GetActorLocation _array_element) (Math|Vector|MakeVector 0.0 0.0 (Variables|Default|GetZAxisLineTraceOffset))) "None"))
    (Utilities|Array|Add (Variables|Default|GetTileWallValues) (Utilities|Struct|MakeTileDataStructure (Utilities|String|Append (Utilities|GetDisplayName _array_element) "_90") (Utilities|GetClass _array_element) _bisnorthwall__2 _biseastwall__2 _bissouthwall__2 _biswestwall__2 90))
    ;[1 1 1] Calculate Wall Values at 180° Rotation
    (Transformation|SetActorRotation _array_element "0,180.000000, 0")
    (bind (_bisnorthwall__3 _biseastwall__3 _bissouthwall__3 _biswestwall__3) (CallFunction|IdentifyTileWalls _array_element (+ (Transformation|GetActorLocation _array_element) (Math|Vector|MakeVector 0.0 0.0 (Variables|Default|GetZAxisLineTraceOffset))) "None"))
    (Utilities|Array|Add (Variables|Default|GetTileWallValues) (Utilities|Struct|MakeTileDataStructure (Utilities|String|Append (Utilities|GetDisplayName _array_element) "_180") (Utilities|GetClass _array_element) _bisnorthwall__3 _biseastwall__3 _bissouthwall__3 _biswestwall__3 180))
    ;[1 1 1] Calculate Wall Values at 270° Rotation
    (Transformation|SetActorRotation _array_element "0,270.000000, 0")
    (bind (_bisnorthwall__4 _biseastwall__4 _bissouthwall__4 _biswestwall__4) (CallFunction|IdentifyTileWalls _array_element (+ (Transformation|GetActorLocation _array_element) (Math|Vector|MakeVector 0.0 0.0 (Variables|Default|GetZAxisLineTraceOffset))) "None"))
    (Utilities|Array|Add (Variables|Default|GetTileWallValues) (Utilities|Struct|MakeTileDataStructure (Utilities|String|Append (Utilities|GetDisplayName _array_element) "_270") (Utilities|GetClass _array_element) _bisnorthwall__4 _biseastwall__4 _bissouthwall__4 _biswestwall__4 270))
    (Transformation|SetActorRotation _array_element) ; Reset rotation to default
  )
  (bind _bsavesuccessful_ (CallFunction|SaveTileWallValuestoCSV (Variables|Default|GetExportedCSVFileName)))
  (if _bsavesuccessful_
    (Development|PrintString "Data Table Saved Sucessfully to 'TileDataTableCSVs' in root of project directory!" true true "(R=0.000000,G=1.000000,B=0.000000,A=1.000000)" 8.0)))

(event Custom|2%20-%20TestLineTrace
  ;[1 1 1] Iterate over TargetTileActors and Call IdentifyTileWalls to Perform Debug Line Trace
  (for _array_element (Variables|Default|GetTargetTileActors)
    (CallFunction|IdentifyTileWalls _array_element (+ (Transformation|GetActorLocation _array_element) (Math|Vector|MakeVector 0.0 0.0 (Variables|Default|GetZAxisLineTraceOffset))) "Persistent")))

(event Custom|3%20-%20Flush%20Debug%20Lines
  (Rendering|Debug|FlushPersistentDebugLines))

(event Custom|1%20-%20Preview%20Line%20Trace%20Range%20with%20Debug%20Lines
  (bind _zaxislinetraceoffset (Variables|Default|GetZAxisLineTraceOffset))
  (bind _zaxislinetraceoffset_2 (Variables|Default|GetZAxisLineTraceOffset))
  ;[1 1 1] For Each Selected Tile, Draw Horizontal & Vertical Debug Line (Length Determined by Value of LineTraceRange)
  (for _array_element (Variables|Default|GetTargetTileActors)
    (Rendering|Debug|DrawDebugLine (+ (Transformation|GetActorLocation _array_element) (Math|Vector|MakeVector (* (Variables|Default|GetLineTraceRange) -1.0) 0.0 _zaxislinetraceoffset_2)) (+ (Transformation|GetActorLocation _array_element) (Math|Vector|MakeVector (Variables|Default|GetLineTraceRange) 0.0 _zaxislinetraceoffset_2)) "(R=1.000000,G=0.000000,B=0.000000,A=1.000000)" 1e+04 5.0)
    (Rendering|Debug|DrawDebugLine (+ (Transformation|GetActorLocation _array_element) (Math|Vector|MakeVector 0.0 (* (Variables|Default|GetLineTraceRange) -1.0) _zaxislinetraceoffset)) (+ (Transformation|GetActorLocation _array_element) (Math|Vector|MakeVector 0.0 (Variables|Default|GetLineTraceRange) _zaxislinetraceoffset)) "(R=1.000000,G=0.000000,B=0.000000,A=1.000000)" 1e+04 5.0)))

(fn ConstructionScript)

(fn IdentifyTileWalls
  (params (TargetTile :type Actor%20Object%20Reference) (LineTraceStartPos :type Vector) (DrawDebugType :type EDrawDebugTrace%20Enum :default "None"))
  (Utilities|FlowControl|Sequence
    (:then_0
      ;[1 1 1] North Wall Line Trace
      (bind _outhit (Collision|LineTraceByChannel LineTraceStartPos (+ LineTraceStartPos (* (Math|Vector|GetForwardVector (Math|Rotator|MakeRotator 0.0 0.0 0.0)) (Variables|Default|GetLineTraceRange))) "TraceTypeQuery1" false 0 DrawDebugType))
      ;[1 1 1] If Hit Target == Target Tile with 0° Rotator, North Wall Hit
      (LocalVariables|SetbNorthWall? (== (.HitActor (Collision|BreakHitResult _outhit)) TargetTile)))
    (:then_1
      ;[1 1 1] East Wall Line Trace
      (bind _outhit_2 (Collision|LineTraceByChannel LineTraceStartPos (+ LineTraceStartPos (* (Math|Vector|GetForwardVector (Math|Rotator|MakeRotator 0.0 0.0 9e+01)) (Variables|Default|GetLineTraceRange))) "TraceTypeQuery1" false 0 DrawDebugType))
      ;[1 1 1] If Hit Target == Target Tile with 90° Rotator, East Wall Hit
      (LocalVariables|SetbEastWall? (== (.HitActor (Collision|BreakHitResult _outhit_2)) TargetTile)))
    (:then_2
      ;[1 1 1] South Wall Line Trace
      (bind _outhit_3 (Collision|LineTraceByChannel LineTraceStartPos (+ LineTraceStartPos (* (Math|Vector|GetForwardVector (Math|Rotator|MakeRotator 0.0 0.0 1.8e+02)) (Variables|Default|GetLineTraceRange))) "TraceTypeQuery1" false 0 DrawDebugType))
      ;[1 1 1] If Hit Target == Target Tile with 180° Rotator, South Wall Hit
      (LocalVariables|SetbSouthWall? (== (.HitActor (Collision|BreakHitResult _outhit_3)) TargetTile)))
    (:then_3
      ;[1 1 1] West Wall Line Trace
      (bind _outhit_4 (Collision|LineTraceByChannel LineTraceStartPos (+ LineTraceStartPos (* (Math|Vector|GetForwardVector (Math|Rotator|MakeRotator 0.0 0.0 2.7e+02)) (Variables|Default|GetLineTraceRange))) "TraceTypeQuery1" false 0 DrawDebugType))
      ;[1 1 1] If Hit Target == Target Tile with 270° Rotator, West Wall Hit
      (LocalVariables|SetbWestWall? (== (.HitActor (Collision|BreakHitResult _outhit_4)) TargetTile)))
    (:then_4
      (return (LocalVariables|GetbNorthWall?) (LocalVariables|GetbEastWall?) (LocalVariables|GetbSouthWall?) (LocalVariables|GetbWestWall?)))))

(fn SaveTileWallValuestoCSV
  (params (CSVFileName :type String))
  (bind _returnvalue (Math|DateTime|Now))
  (bind (_year _month _day _hour _minute _second) (Math|DateTime|BreakDateTime _returnvalue))
  ;[1 1 1] Check Length of Tile Wall Values Array
  (Math|Integer|CompareInt (Utilities|Array|Length (Variables|Default|GetTileWallValues))
    (:>
      ;[1 1 1] Clear TileStringData Array Used for Serialisation & Add First Entry (used for Data Structure Headers)
      (Utilities|Array|Clear (LocalVariables|GetTileStringData))
      (Utilities|Array|Add (LocalVariables|GetTileStringData) "---,TileName,TileActor,NorthWall?,EastWall?,SouthWall?,WestWall?,Rotation")
      ;[1 1 1] Iterate over TileWallValues Array and
      (for (_array_element _array_index) (Variables|Default|GetTileWallValues)
        (Utilities|Array|Add (LocalVariables|GetTileStringData) (Utilities|String|Append (Utilities|String|ToString(Integer) _array_index) "," (.TileName (Utilities|Struct|BreakTileDataStructure _array_element)) "," (Utilities|GetClassDisplayName (.TileActor (Utilities|Struct|BreakTileDataStructure _array_element))) "," (Utilities|String|ToString(Boolean) (.NorthWall? (Utilities|Struct|BreakTileDataStructure _array_element))) "," (Utilities|String|ToString(Boolean) (.EastWall? (Utilities|Struct|BreakTileDataStructure _array_element))) "," (Utilities|String|ToString(Boolean) (.SouthWall? (Utilities|Struct|BreakTileDataStructure _array_element))) "," (Utilities|String|ToString(Boolean) (.WestWall? (Utilities|Struct|BreakTileDataStructure _array_element))) "," (Utilities|String|ToString(Integer) (.Rotation (Utilities|Struct|BreakTileDataStructure _array_element))))))
      (if (Utilities|Array|IsEmpty CSVFileName)
        (bind _returnvalue_2 (Class|TextFileManager|SaveArrayText (Utilities|String|Append (Class|KismetSystemLibrary|GetProjectDirectory) "\\TileDataTableCSVs") (Utilities|String|Append "TILE_" (Utilities|String|ToString(Integer) _year) "_" (Utilities|String|ToString(Integer) _month) "_" (Utilities|String|ToString(Integer) _day) "_" (Utilities|String|ToString(Integer) _hour) "_" (Utilities|String|ToString(Integer) _minute) "_" (Utilities|String|ToString(Integer) _second) ".csv") (LocalVariables|GetTileStringData) true))
        (return _returnvalue_2)
        (else
          ;[1 1 1] Check if Provided File Name Ends in .csv
          (if (Utilities|String|EndsWith CSVFileName ".csv")
            (bind _returnvalue_3 (Class|TextFileManager|SaveArrayText (Utilities|String|Append (Class|KismetSystemLibrary|GetProjectDirectory) "\\TileDataTableCSVs") "" (LocalVariables|GetTileStringData) true))
            (return _returnvalue_3)
            (else
              (bind _returnvalue_4 (Class|TextFileManager|SaveArrayText (Utilities|String|Append (Class|KismetSystemLibrary|GetProjectDirectory) "\\TileDataTableCSVs") (Utilities|String|Append CSVFileName ".csv") (LocalVariables|GetTileStringData) true))
              (return _returnvalue_4))))))
    (:==
      _)
    (:<
      _))
  (Development|PrintString "ERROR! Tile Wall Values array is empty - there is no valid data to save!" true true "(R=1.000000,G=0.000000,B=0.000000,A=1.000000)" 8.0)
  (return false))