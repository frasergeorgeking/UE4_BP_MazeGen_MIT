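; Maze controller that procedurally generates a grid maze and spawns it as tile actors.
; GenerateMaze runs the Sidewinder algorithm on a flat wall array, syncs neighbouring walls, matches cells to data table tiles, then spawns and rotates them row by row.
; When a CSV data table is supplied, it maps that layout to tiles instead of generating one.
; SaveGeneratedMazeAsCSV exports selected tiles to a timestamped CSV through a custom C++ node.
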(event Custom|GenerateMaze
  (bind _currentrun (Variables|Default|GetCurrentRun))
  (bind _width (Variables|Default|GetWidth))
  (bind _tiledatastructureref (Variables|Default|GetTileDataStructureRef))
  (bind _width_2 (Variables|Default|GetWidth))
  (bind _width_3 (Variables|Default|GetWidth))
  (bind _tilewallvalues (Variables|Default|GetTileWallValues))
  (bind _importeddatatable (Variables|Default|GetImportedDataTable))
  (bind _width_4 (Variables|Default|GetWidth))
  (bind _tilewallvalues_2 (Variables|Default|GetTileWallValues))
  (bind (_tilename _tileactor _northwall_ _eastwall_ _southwall_ _westwall_ _rotation) (Utilities|Struct|BreakTileDataStructure _tiledatastructureref))
  (bind _returnvalue (Utilities|Array|LastIndex _currentrun))
  (bind _returnvalue_2 (Utilities|Array|LastIndex _tilewallvalues))
  (bind _returnvalue_3 (Math|Random|RandomIntegerinRange 0 _returnvalue))
  (bind _output (Utilities|Array|Get(acopy) _tilewallvalues _returnvalue_2))
  (bind (_tilename_2 _tileactor_2 _northwall__2 _eastwall__2 _southwall__2 _westwall__2 _rotation_2) (Utilities|Struct|BreakTileDataStructure _output))
  (bind _output_2 (Utilities|Array|Get(acopy) _currentrun _returnvalue_3))
  (bind _output_3 (Utilities|Array|Get(acopy) _tilewallvalues_2 _output_2))
  (bind (_tilename_3 _tileactor_3 _northwall__3 _eastwall__3 _southwall__3 _westwall__3 _rotation_3) (Utilities|Struct|BreakTileDataStructure _output_3))
  ;[1 1 1] Destroy all Currently Spawned Tiles & Reset Variables
  (CallFunction|RemoveSpawnedTiles)
  (CallFunction|ResetVariables)
  ;[1 1 1] Check if a CSV has been Imported
  (if (Utilities|IsValid (Variables|Default|GetImportedDataTable))
    (Development|PrintString "Imported CSV Detected")
    ;[1 1 1] For Every Row in Imported Data Table, Create Entry in 'Imported CSV Wall Values' Array
    (bind _outrownames (DataTable|GetDataTableRowNames _importeddatatable))
    (for _array_element _outrownames
      (bind _returnvalue_4 (Utilities|GetDataTableRow _importeddatatable _array_element)
        (:then
          (Utilities|Array|Add (Variables|Default|GetImportedCSVWallValues) (Utilities|Struct|MakeTileCSVDataStructure (.NorthWall? (Utilities|Struct|BreakTileCSVDataStructure _returnvalue_4)) (.EastWall? (Utilities|Struct|BreakTileCSVDataStructure _returnvalue_4)) (.SouthWall? (Utilities|Struct|BreakTileCSVDataStructure _returnvalue_4)) (.WestWall? (Utilities|Struct|BreakTileCSVDataStructure _returnvalue_4)) (.X (Utilities|Struct|BreakTileCSVDataStructure _returnvalue_4)) (.Y (Utilities|Struct|BreakTileCSVDataStructure _returnvalue_4)) (.TileName (Utilities|Struct|BreakTileCSVDataStructure _returnvalue_4)) (.Rotation (Utilities|Struct|BreakTileCSVDataStructure _returnvalue_4)))))))
    ;[1 1 1] Convert CSV Data Structure to Main Tile Data Structure and Write to Selected Tiles Array
    (bind _outputpin (|MapCSVDataStructuretoSelectedTilesArray))
    (else
      (Development|PrintString "No Imported CSV Detected. Spawning new Maze!")
      ;[1 1 1] Set 'TotalTiles'
      (Variables|Default|SetTotalTiles (* (Variables|Default|GetWidth) (Variables|Default|GetHeight)))
      ;[1 1 1] For each tile, create an entry in the tile data structure array and initialise all wall values to 1111 (North, East, South, West)
      (for _index (range 0 (- (Variables|Default|GetTotalTiles) 1)) ; Loops against total number of tiles - ensures each tile has its own position in array
        (Utilities|Array|Add (Variables|Default|GetTileWallValues) (Utilities|Struct|MakeTileDataStructure _tilename _tileactor true true true true _rotation)) ; Add initialised TileDataStructure\nentries to array
      )
      ;[1 1 1] Run Sidewinder Algorithm Against Wall Tile Array
      (for (_array_element_2 _array_index) (Variables|Default|GetTileWallValues)
        ;;[1 1 1] Add Cell to Current Run
        (Utilities|Array|Add (Variables|Default|GetCurrentRun) _array_index)
        ;;[1 1 1] Check if Current Cell is on North Border of Maze, if so Always Remove East Wall of Cell
        (Math|Integer|CompareInt (|(i/MazeWidth) _array_index (Variables|Default|GetWidth)) (- (Variables|Default|GetHeight) 1) ; If Y == (Height -1), the cell\nis on the North Border
          (:>
            ;;[1 1 1] Check if Current Cell is on East Border of Maze, if so Always Close the Run
            (Math|Integer|CompareInt (|(i%MazeWidth) _array_index _width_2) (- _width_2 1) :!label _label ; If X == (Width -1), the cell\nis on the East Border
              (:>
                ;;[1 1 1] If on Neither Border, Randomly Select
                ;; an Option
                (if (Math|Random|RandomBool) :!label _label_2
                  (Utilities|Array|SetArrayElem (Variables|Default|GetTileWallValues) _array_index (Utilities|Struct|MakeTileDataStructure (.TileName (Utilities|Struct|BreakTileDataStructure _array_element_2)) (.TileActor (Utilities|Struct|BreakTileDataStructure _array_element_2)) (.NorthWall? (Utilities|Struct|BreakTileDataStructure _array_element_2)) false (.SouthWall? (Utilities|Struct|BreakTileDataStructure _array_element_2)) (.WestWall? (Utilities|Struct|BreakTileDataStructure _array_element_2)) (.Rotation (Utilities|Struct|BreakTileDataStructure _array_element_2))) :!label _label_3)
                  (else
                    (Utilities|Array|SetArrayElem (Variables|Default|GetTileWallValues) _output_2 (Utilities|Struct|MakeTileDataStructure _tilename_3 _tileactor_3 false _eastwall__3 _southwall__3 _westwall__3 _rotation_3) :!label _label_4)
                    (Utilities|Array|Clear (Variables|Default|GetCurrentRun)) ; Closes the run and \nclears the array
                  )))
              (:==
                (goto _label_4))
              (:<
                (goto _label_2))))
          (:==
            (goto _label_3))
          (:<
            (goto _label))))
      ;[1 1 1] Manually Update the Wall Values of the Final Cell (always the Top-Right Cell)
      (Utilities|Array|SetArrayElem _tilewallvalues _returnvalue_2 (Utilities|Struct|MakeTileDataStructure _tilename_2 _tileactor_2 true true true true _rotation_2))
      (for (_array_element_3 _array_index_2) (Variables|Default|GetTileWallValues)
        ;[1 1 1] Check if each Cell is Missing a North Wall
        (if (Math|Boolean|Equal(Boolean) (.NorthWall? (Utilities|Struct|BreakTileDataStructure _array_element_3)) false)
          ;[1 1 1] Log Each Affected North Neighbour Cell
          (Utilities|Array|Add (Variables|Default|GetAffectedNorthNeighbourArray) (Utilities|Struct|MakeAffectedNeighbourDataStructure (|(x+(MazeWidth*y)) (|(i%MazeWidth) _array_index_2 _width) _width (+ (|(i/MazeWidth) _array_index_2 _width) 1)) false true))))
      ;[1 1 1] Update Wall Values of all Affected Neighbour Cells (North)
      (for _array_element_4 (Variables|Default|GetAffectedNorthNeighbourArray)
        (Utilities|Array|SetArrayElem (Variables|Default|GetTileWallValues) (.AffectedCellIndexPos (Utilities|Struct|BreakAffectedNeighbourDataStructure _array_element_4)) (Utilities|Struct|MakeTileDataStructure (.TileName (Utilities|Struct|BreakTileDataStructure (Utilities|Array|Get(acopy) (Variables|Default|GetTileWallValues) (.AffectedCellIndexPos (Utilities|Struct|BreakAffectedNeighbourDataStructure _array_element_4))))) (.TileActor (Utilities|Struct|BreakTileDataStructure (Utilities|Array|Get(acopy) (Variables|Default|GetTileWallValues) (.AffectedCellIndexPos (Utilities|Struct|BreakAffectedNeighbourDataStructure _array_element_4))))) (.NorthWall? (Utilities|Struct|BreakTileDataStructure (Utilities|Array|Get(acopy) (Variables|Default|GetTileWallValues) (.AffectedCellIndexPos (Utilities|Struct|BreakAffectedNeighbourDataStructure _array_element_4))))) (.EastWall? (Utilities|Struct|BreakTileDataStructure (Utilities|Array|Get(acopy) (Variables|Default|GetTileWallValues) (.AffectedCellIndexPos (Utilities|Struct|BreakAffectedNeighbourDataStructure _array_element_4))))) false (.WestWall? (Utilities|Struct|BreakTileDataStructure (Utilities|Array|Get(acopy) (Variables|Default|GetTileWallValues) (.AffectedCellIndexPos (Utilities|Struct|BreakAffectedNeighbourDataStructure _array_element_4))))) (.Rotation (Utilities|Struct|BreakTileDataStructure (Utilities|Array|Get(acopy) (Variables|Default|GetTileWallValues) (.AffectedCellIndexPos (Utilities|Struct|BreakAffectedNeighbourDataStructure _array_element_4))))))))
      (for (_array_element_5 _array_index_3) (Variables|Default|GetTileWallValues)
        ;[1 1 1] Check if each Cell is Missing a North Wall
        (if (Math|Boolean|Equal(Boolean) (.EastWall? (Utilities|Struct|BreakTileDataStructure _array_element_5)) false)
          ;[1 1 1] Log Each Affected North Neighbour Cell
          (Utilities|Array|Add (Variables|Default|GetAffectedEastNeighbourArray) (Utilities|Struct|MakeAffectedNeighbourDataStructure (|(x+(MazeWidth*y)) (+ (|(i%MazeWidth) _array_index_3 _width_3) 1) _width_3 (|(i/MazeWidth) _array_index_3 _width_3)) true false))))
      ;[1 1 1] Update Wall Values of all Affected Neighbour Cells (East)
      (for _array_element_6 (Variables|Default|GetAffectedEastNeighbourArray)
        (Utilities|Array|SetArrayElem (Variables|Default|GetTileWallValues) (.AffectedCellIndexPos (Utilities|Struct|BreakAffectedNeighbourDataStructure _array_element_6)) (Utilities|Struct|MakeTileDataStructure (.TileName (Utilities|Struct|BreakTileDataStructure (Utilities|Array|Get(acopy) (Variables|Default|GetTileWallValues) (.AffectedCellIndexPos (Utilities|Struct|BreakAffectedNeighbourDataStructure _array_element_6))))) (.TileActor (Utilities|Struct|BreakTileDataStructure (Utilities|Array|Get(acopy) (Variables|Default|GetTileWallValues) (.AffectedCellIndexPos (Utilities|Struct|BreakAffectedNeighbourDataStructure _array_element_6))))) (.NorthWall? (Utilities|Struct|BreakTileDataStructure (Utilities|Array|Get(acopy) (Variables|Default|GetTileWallValues) (.AffectedCellIndexPos (Utilities|Struct|BreakAffectedNeighbourDataStructure _array_element_6))))) (.EastWall? (Utilities|Struct|BreakTileDataStructure (Utilities|Array|Get(acopy) (Variables|Default|GetTileWallValues) (.AffectedCellIndexPos (Utilities|Struct|BreakAffectedNeighbourDataStructure _array_element_6))))) (.SouthWall? (Utilities|Struct|BreakTileDataStructure (Utilities|Array|Get(acopy) (Variables|Default|GetTileWallValues) (.AffectedCellIndexPos (Utilities|Struct|BreakAffectedNeighbourDataStructure _array_element_6))))) false (.Rotation (Utilities|Struct|BreakTileDataStructure (Utilities|Array|Get(acopy) (Variables|Default|GetTileWallValues) (.AffectedCellIndexPos (Utilities|Struct|BreakAffectedNeighbourDataStructure _array_element_6))))))))
      ;[1 1 1] Find Compatible Tile for each Entry in Tile Wall Values Array
      (for (_array_element_7 _array_index_4) (Variables|Default|GetTileWallValues)
        (CallFunction|FindTileinDataTable _array_element_7 _array_index_4) ; Runs comparison against tile wall values at any given index to tile data table\nand adds reference to 'Selected Tiles' array
      )
      ;[1 1 1] Verifies Length of 'Tile Wall Values' and 'Selected Tiles' Arrays Match - i.e. a tile has been found for each index position in main array
      (Math|Integer|CompareInt (Utilities|Array|Length (Variables|Default|GetSelectedTiles)) (Utilities|Array|Length (Variables|Default|GetTileWallValues))
        (:==
          ;[1 1 1] Loop Through 'SelectedTiles' Array, Spawn Required Actor at Given Transform and Log All Transforms in 'TileSpawnTransforms' Array
          (for (_array_element_8 _array_index_5) (Variables|Default|GetSelectedTiles)
            (bind _returnvalue_5 (Game|SpawnActorfromClass (.TileActor (Utilities|Struct|BreakTileDataStructure _array_element_8)) (Variables|Default|GetMazeSpawnTransform) "Undefined" 0 0))
            (Utilities|Array|Add (Variables|Default|GetSpawnedTiles) _returnvalue_5)
            (Utilities|Array|Add (Variables|Default|GetTileSpawnTransforms) (Variables|Default|GetMazeSpawnTransform))
            ;[1 1 1] Perform East Border Lookup on each Array Index
            (Math|Integer|CompareInt (|(i%MazeWidth) _array_index_5 _width_4) (- _width_4 1)
              (:>
                ;[1 1 1] If not on East Border, offset in the YAxis
                ; (Note: Y is relative to world space, *NOT* 1D to 2D Array Lookups)
                (bind _updatedspawntransform (CallFunction|CalculateYSpawningOffset (Variables|Default|GetMazeSpawnTransform) :!label _label_5))
                (Variables|Default|SetMazeSpawnTransform _updatedspawntransform))
              (:==
                ;[1 1 1] If on East Border, Perform 1D to 2D Lookup to Return Required Index Number
                (bind _updatedspawntransform_2 (CallFunction|CalculateXSpawningOffset (Utilities|Array|Get(acopy) (Variables|Default|GetTileSpawnTransforms) (|(x+(MazeWidth*y)) 0 (Variables|Default|GetWidth) (Variables|Default|GetSpawningYRef)))))
                (Variables|Default|SetMazeSpawnTransform _updatedspawntransform_2)
                ;[1 1 1] Increment Value of Y Spawning Ref for Next Row
                (bind _result (Math|Integer|IncrementInt (Variables|Default|GetSpawningYRef))
                  (:%20%20
                    (Variables|Default|SetSpawningYRef _result))))
              (:<
                (goto _label_5))))
          ;[1 1 1] Rotate Spawned Tiles to Connect Maze
          (for (_array_element_9 _array_index_6) (Variables|Default|GetSpawnedTiles)
            (Transformation|SetActorRotation _array_element_9 (Math|Rotator|MakeRotator 0.0 0.0 (Math|Conversions|ToFloat(Integer) (.Rotation (Utilities|Struct|BreakTileDataStructure (Utilities|Array|Get(acopy) (Variables|Default|GetSelectedTiles) _array_index_6))))))))
        (:<
          (Development|PrintString "Array sizes different, tile match not found for one or more index positions!"))))))

(event Custom|Destroy%20Spawned%20Tiles
  ;[1 1 1] Destroy all Currently Spawned Tiles & Reset Variables
  (CallFunction|RemoveSpawnedTiles)
  (CallFunction|ResetVariables))

(fn ConstructionScript)

(fn EastBorderLookup
  (params (Width :type Integer) (X :type Integer))
  ;[1 1 1] If X == (Width - 1), set IsEastBorder? to True
  (if (== X (- Width 1))
    ;;[1 1 1] Updates 'IsEastBorder?' Bool
    (Variables|Default|SetIsOnEastBorder? true)
    (else
      (Variables|Default|SetIsOnEastBorder? false)))
  (return))

(fn NorthBorderLookup
  (params (Height :type Integer) (Y :type Integer))
  ;[1 1 1] If Y == (Height - 1), set IsNorthBorder? to True
  (if (== (- Height 1) Y)
    ;;[1 1 1] Updates 'IsNorthBorder?' Bool
    (Variables|Default|SetIsOnNorthBorder? true)
    (else
      (Variables|Default|SetIsOnNorthBorder? false)))
  (return))

(fn NorthEastBorderLookup
  (params (Width :type Integer) (Height :type Integer) (X :type Integer) (Y :type Integer))
  ;[1 1 1] If X == (Width - 1) AND Y == (Height - 1), set 'IsNorthEastBorder' to True
  (if (== Y (- Height 1))
    (if (== X (- Width 1))
      (Variables|Default|SetIsNorthEastBorder? true)
      (else
        (Variables|Default|SetIsNorthEastBorder? false :!label _label)))
    (else
      (goto _label)))
  (return))

(fn FindTileinDataTable
  (params (CurrentTileRequirements :type Tile%20Data%20Structure%20Structure) (CurrentTileIndexPosition :type Integer))
  (bind (_tilename _tileactor _northwall_ _eastwall_ _southwall_ _westwall_) (Utilities|Struct|BreakTileDataStructure CurrentTileRequirements))
  (bind _allvalidtiles (LocalVariables|GetAllValidTiles))
  (bind _allvalidtiles_2 (LocalVariables|GetAllValidTiles))
  (bind _returnvalue (Utilities|Array|LastIndex _allvalidtiles))
  (bind _returnvalue_2 (Math|Random|RandomIntegerinRange 0 _returnvalue))
  (bind _output (Utilities|Array|Get(acopy) _allvalidtiles_2 _returnvalue_2))
  ;[1 1 1] Loop Through Each Data Table Row Entry
  (bind _outrownames (DataTable|GetDataTableRowNames (Variables|Default|GetTileDataTableToSpawn)))
  (for _array_element _outrownames
    (bind _returnvalue_3 (Utilities|GetDataTableRow (Variables|Default|GetTileDataTableToSpawn) _array_element)
      (:then
        ;[1 1 1] If Valid Tile Is Found, Add to 'AllValidTiles' Local Array
        (if (Math|Boolean|Equal(Boolean) (.NorthWall? (Utilities|Struct|BreakTileDataStructure _returnvalue_3)) _northwall_)
          (if (Math|Boolean|Equal(Boolean) (.EastWall? (Utilities|Struct|BreakTileDataStructure _returnvalue_3)) _eastwall_)
            (if (Math|Boolean|Equal(Boolean) (.SouthWall? (Utilities|Struct|BreakTileDataStructure _returnvalue_3)) _southwall_)
              (if (Math|Boolean|Equal(Boolean) (.WestWall? (Utilities|Struct|BreakTileDataStructure _returnvalue_3)) _westwall_)
                (Utilities|Array|Add (LocalVariables|GetAllValidTiles) _returnvalue_3)
                ;[1 1 1] Add to 'SelectedTiles' Main Array
                (Utilities|Array|Add (Variables|Default|GetSelectedTiles) _output)
                (return _output)))))))))

(fn CalculateTileRotationZ
  (params (TileDataStructureInputRef :type Tile%20Data%20Structure%20Structure))
  ;[1 1 1] Creates Rotation Offset Output used for Calculating Spawn Transform of Tiles
  (return (Math|Vector|MakeVector 0.0 0.0 (Math|Conversions|ToFloat(Integer) (.Rotation (Utilities|Struct|BreakTileDataStructure TileDataStructureInputRef))))))

(fn CalculateYSpawningOffset
  (params (InputTransform :type Transform))
  (bind (_location _rotation _scale) (Math|Transform|BreakTransform InputTransform))
  (bind (_x _y _z) (Math|Vector|BreakVector _location))
  (return (Math|Transform|MakeTransform (Math|Vector|MakeVector _x (+ (Math|Conversions|ToFloat(Integer) (Variables|Default|GetTileWidthInUnits)) _y) _z) _rotation _scale)) ; Outputs Updated Spawn Transform
)

(fn CalculateXSpawningOffset
  (params (InputTransform :type Transform))
  (bind (_location _rotation _scale) (Math|Transform|BreakTransform InputTransform))
  (bind (_x _y _z) (Math|Vector|BreakVector _location))
  (return (Math|Transform|MakeTransform (Math|Vector|MakeVector (+ (Math|Conversions|ToFloat(Integer) (Variables|Default|GetTileWidthInUnits)) _x) _y _z) _rotation _scale)) ; Outputs Updated Spawn Transform
)

(fn SelectFinalCell
  (bind _width (Variables|Default|GetWidth))
  (bind _potential_cell_spawn_index_positions (LocalVariables|GetPotential%20Cell%20Spawn%20Index%20Positions))
  ;[1 1 1] X and Y Value Lookup on Each Index Position
  (for (_ _array_index) (Variables|Default|GetSelectedTiles)
    (LocalVariables|SetLocalYRef (|(i/MazeWidth) _array_index _width))
    (LocalVariables|SetLocalXRef (|(i%MazeWidth) _array_index _width))
    ;[1 1 1] Is Cell on East Border?
    (if (== (LocalVariables|GetLocalXRef) (- (Variables|Default|GetWidth) 1))
      ;[1 1 1] If True, Add to Local Cell Tracking Array
      (Utilities|Array|Add (LocalVariables|GetPotential%20Cell%20Spawn%20Index%20Positions) _array_index)
      (else
        ;[1 1 1] Is Cell on East Border -1?
        (if (== (LocalVariables|GetLocalXRef) (- (Variables|Default|GetWidth) 2))
          ;[1 1 1] If True, Add to Local Cell Tracking Array
          (Utilities|Array|Add (LocalVariables|GetPotential%20Cell%20Spawn%20Index%20Positions) _array_index)
          (else
            ;[1 1 1] Is Cell on North Border?
            (if (== (LocalVariables|GetLocalYRef) (- (Variables|Default|GetHeight) 1))
              ;[1 1 1] If True, Add to Local Cell Tracking Array
              (Utilities|Array|Add (LocalVariables|GetPotential%20Cell%20Spawn%20Index%20Positions) _array_index)
              (else
                ;[1 1 1] Is Cell on North Border - 1?
                (if (== (LocalVariables|GetLocalYRef) (- (Variables|Default|GetHeight) 2))
                  ;[1 1 1] If True, Add to Local Cell Tracking Array
                  (Utilities|Array|Add (LocalVariables|GetPotential%20Cell%20Spawn%20Index%20Positions) _array_index)))))))))
  (return (Utilities|Array|Get(acopy) _potential_cell_spawn_index_positions (Math|Random|RandomInteger (Utilities|Array|LastIndex _potential_cell_spawn_index_positions)))))

(fn SaveGeneratedMazeasCSV
  (bind _returnvalue (Math|DateTime|Now))
  (bind _tiledatavaluesstring (Variables|Default|GetTileDataValuesString))
  (bind (_year _month _day _hour _minute _second) (Math|DateTime|BreakDateTime _returnvalue))
  (for (_array_element _array_index) (Variables|Default|GetSelectedTiles)
    (Utilities|Array|Add _tiledatavaluesstring (Utilities|String|Append (Utilities|String|ToString(Integer) _array_index) "," (Utilities|String|ToString(Boolean) (.NorthWall? (Utilities|Struct|BreakTileDataStructure _array_element))) "," (Utilities|String|ToString(Boolean) (.EastWall? (Utilities|Struct|BreakTileDataStructure _array_element))) "," (Utilities|String|ToString(Boolean) (.SouthWall? (Utilities|Struct|BreakTileDataStructure _array_element))) "," (Utilities|String|ToString(Boolean) (.WestWall? (Utilities|Struct|BreakTileDataStructure _array_element))) "," (Utilities|String|ToString(Integer) (|(i%MazeWidth) _array_index (Variables|Default|GetWidth))) "," (Utilities|String|ToString(Integer) (|(i/MazeWidth) _array_index (Variables|Default|GetWidth))) "," (.TileName (Utilities|Struct|BreakTileDataStructure _array_element)) "," (Utilities|String|ToString(Integer) (.Rotation (Utilities|Struct|BreakTileDataStructure _array_element))))))
  (Class|TextFileManager|SaveArrayText (Utilities|String|Append (Class|KismetSystemLibrary|GetProjectDirectory) "\\MazeCSVExports") (Utilities|String|Append "MAZECSVEXPO_" (Utilities|String|RightChop (Utilities|GetObjectName (Variables|Default|GetTileDataTableToSpawn)) 5) "_" (Utilities|String|ToString(Integer) _year) "_" (Utilities|String|ToString(Integer) _month) "_" (Utilities|String|ToString(Integer) _day) "_" (Utilities|String|ToString(Integer) _hour) "_" (Utilities|String|ToString(Integer) _minute) "_" (Utilities|String|ToString(Integer) _second) ".csv") _tiledatavaluesstring false) ; Custom C++ node written to call built-in string\nexporting; not supported in blueprint by default \n(but present in the engine)
  (return (Variables|Default|GetTileDataValuesString)) ; Outputs reference to array for debugging
)

(fn ConvertCSVDataStucture
  (params (ArrayToConvert :type Array%20of%20Tile%20CSV%20Data%20Structure%20Structures))
  (Utilities|Array|Clear (Variables|Default|GetTileWallValues)) ; Ensures array is empty before\nentries are written
  (for (_array_element _array_index) ArrayToConvert
    (Utilities|Array|SetArrayElem (Variables|Default|GetTileWallValues) _array_index (Utilities|Struct|MakeTileDataStructure "" 0 (.NorthWall? (Utilities|Struct|BreakTileCSVDataStructure _array_element)) (.EastWall? (Utilities|Struct|BreakTileCSVDataStructure _array_element)) (.SouthWall? (Utilities|Struct|BreakTileCSVDataStructure _array_element)) (.WestWall? (Utilities|Struct|BreakTileCSVDataStructure _array_element))) true) ; Ensures index positions\nremain identical across\narrays
  )
  (return))

(fn ResetVariables
  (Variables|Default|SetMazeSpawnTransform (Math|Transform|MakeTransform "0, 0, 0"))
  (Variables|Default|SetSpawningYRef 0)
  (Utilities|Array|Clear (Variables|Default|GetTileWallValues))
  (Utilities|Array|Clear (Variables|Default|GetAffectedNorthNeighbourArray))
  (Utilities|Array|Clear (Variables|Default|GetAffectedEastNeighbourArray))
  (Utilities|Array|Clear (Variables|Default|GetSelectedTiles))
  (Utilities|Array|Clear (Variables|Default|GetTileSpawnTransforms))
  (Utilities|Array|Clear (Variables|Default|GetImportedCSVWallValues))
  (Utilities|Array|Clear (Variables|Default|GetTileDataValuesString))
  (Utilities|Array|Clear (Variables|Default|GetCurrentRun)))

(fn RemoveSpawnedTiles
  (bind _spawnedtiles (Variables|Default|GetSpawnedTiles))
  (for _array_element _spawnedtiles
    (Actor|DestroyActor _array_element))
  (Utilities|Array|Clear _spawnedtiles))